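; PlayerPawnBP is the player pawn in a space RTS, showing the commander's body and command throne according to settings held in GameInstanceSpaceRTS.
; On BeginPlay it binds to the game instance's player-pawn-changed event, and both startup and that event read the body visibility and position settings.
; UpdateBodyPosition toggles body visibility, then uses the position to swap the commander mesh and show or hide the throne and its emperor add-on.
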(event Custom|OnPlayerPawnChanged
  (bind _asgame_instance_space_rts (Utilities|Casting|CastToGameInstanceSpaceRTS (Game|GetGameInstance)))
  (CallFunction|UpdateBodyPosition (Variables|/Script/SpaceRTS.GameInstanceSpaceRTS|GetShowPlayerPawnBody _asgame_instance_space_rts) (Variables|/Script/SpaceRTS.GameInstanceSpaceRTS|GetPlayerBodyPosition _asgame_instance_space_rts)))

(event EventBeginPlay
  (bind _returnvalue (Game|GetGameInstance))
  (bind _asgame_instance_space_rts (Utilities|Casting|CastToGameInstanceSpaceRTS _returnvalue))
  (EventDispatchers|BindEventtoOnPlayerPawnChanged _asgame_instance_space_rts (delegate Custom|OnPlayerPawnChanged))
  (bind _asgame_instance_space_rts_2 (Utilities|Casting|CastToGameInstanceSpaceRTS _returnvalue))
  (CallFunction|UpdateBodyPosition (Variables|/Script/SpaceRTS.GameInstanceSpaceRTS|GetShowPlayerPawnBody _asgame_instance_space_rts_2) (Variables|/Script/SpaceRTS.GameInstanceSpaceRTS|GetPlayerBodyPosition _asgame_instance_space_rts_2)))

(fn ConstructionScript)

(fn UpdateBodyPosition
  (params (CurrentShowPlayerBody :type Boolean) (CurrentBodyPosition :type EPlayerBodyPosition%20Enum))
  (Rendering|SetVisibility (Variables|Default|GetPlayerBody) CurrentShowPlayerBody false)
  (switch Utilities|FlowControl|Switch|SwitchonEPlayerBodyPosition CurrentBodyPosition
    (:Standing
      (Rendering|SetVisibility (Variables|Default|GetCommandThrone) false false)
      (Rendering|SetVisibility (Variables|Default|GetCommandThroneEmporerAddon) false false)
      (Components|StaticMesh|SetStaticMesh (Variables|Default|GetPlayerBody) "/Game/Actors/PlayerPawnBP/Meshes/Male_Commander_Standing_Pointing_Reduced.Male_Commander_Standing_Pointing_Reduced"))
    (:NormalChair
      (Rendering|SetVisibility (Variables|Default|GetCommandThrone) true false)
      (Rendering|SetVisibility (Variables|Default|GetCommandThroneEmporerAddon) false false)
      (Components|StaticMesh|SetStaticMesh (Variables|Default|GetPlayerBody) "/Game/Actors/PlayerPawnBP/Meshes/Male_Commander_Normal_Reduced.Male_Commander_Normal_Reduced"))
    (:SwivelChair
      (Rendering|SetVisibility (Variables|Default|GetCommandThrone) true false)
      (Rendering|SetVisibility (Variables|Default|GetCommandThroneEmporerAddon) false false)
      (Components|StaticMesh|SetStaticMesh (Variables|Default|GetPlayerBody) "/Game/Actors/PlayerPawnBP/Meshes/Male_Commander_Normal_Reduced.Male_Commander_Normal_Reduced"))
    (:EmporerChair
      (Rendering|SetVisibility (Variables|Default|GetCommandThrone) true false)
      (Rendering|SetVisibility (Variables|Default|GetCommandThroneEmporerAddon) true false)
      (Components|StaticMesh|SetStaticMesh (Variables|Default|GetPlayerBody) "/Game/Actors/PlayerPawnBP/Meshes/Male_Commander_Emporer_Reduced.Male_Commander_Emporer_Reduced"))))