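; Player pawn for an interaction test that drives a head-tracked gaze reticle and updates an FPS counter widget.
; Each tick, the camera follows headset rotation when an HMD is enabled and casts a trace from the pawn along its forward vector.
; The reticle moves to the hit or default distance, scaling proportionally with it.
; Hitting a SteeringAgentPawn plays its animation once, re-armed only when the trace hits nothing.
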(event EventTick
  (params (DeltaSeconds :type Float%20%28single-precision%29))
  (bind _returnvalue (Transformation|GetActorLocation))
  (bind _recticle (Variables|Default|GetRecticle))
  (bind _defaultrectiledistance (Variables|Default|GetDefaultRectileDistance))
  (bind _returnvalue_2 (/ _defaultrectiledistance 3e+03))
  (bind _aswidget_fps (Utilities|Casting|CastToWidget_FPS (UserInterface|GetUserWidgetObject (Variables|Default|GetWidget))))
  (Default|TickFPSCounter _aswidget_fps)
  (if (Class|HeadMountedDisplayFunctionLibrary|IsHeadMountedDisplayEnabled)
    (Transformation|SetRelativeRotation (Variables|Default|GetCamera) (.DeviceRotation (Class|HeadMountedDisplayFunctionLibrary|GetOrientationandPosition)) false))
  (bind _outhit (Collision|LineTraceByChannel _returnvalue (+ _returnvalue (* (Math|Vector|GetForwardVector (Variables|Default|GetCamera)) 2e+04)) "TraceTypeQuery2" false 0 "None"))
  (if (.bBlockingHit (Collision|BreakHitResult _outhit))
    (Transformation|SetRelativeScale3D _recticle (Math|Vector|MakeVector (/ (Math|Vector|VectorLength (- (.ImpactPoint (Collision|BreakHitResult _outhit)) (.TraceStart (Collision|BreakHitResult _outhit)))) 3e+03) (/ (Math|Vector|VectorLength (- (.ImpactPoint (Collision|BreakHitResult _outhit)) (.TraceStart (Collision|BreakHitResult _outhit)))) 3e+03) (/ (Math|Vector|VectorLength (- (.ImpactPoint (Collision|BreakHitResult _outhit)) (.TraceStart (Collision|BreakHitResult _outhit)))) 3e+03)))
    (Transformation|SetRelativeLocation _recticle (Math|Vector|MakeVector (Math|Vector|VectorLength (- (.ImpactPoint (Collision|BreakHitResult _outhit)) (.TraceStart (Collision|BreakHitResult _outhit)))) 0.0 0.0) true)
    (Utilities|Casting|CastToSteeringAgentPawn (.HitActor (Collision|BreakHitResult _outhit)))
    (Utilities|FlowControl|DoOnce false :!label _label
      (:Completed
        (Components|Timeline|SetPlayRate _recticle 2.0)
        (Components|Timeline|SetLooping _recticle false)
        (Components|Timeline|PlayfromStart _recticle)))
    (else
      (Components|Timeline|SetPlaybackPosition _recticle 0.0 false)
      (Audio|Components|Audio|Stop (Variables|Default|GetRecticle))
      (Transformation|SetRelativeLocation _recticle (Math|Vector|MakeVector _defaultrectiledistance 0.0 0.0) true)
      (Transformation|SetRelativeScale3D _recticle (Math|Vector|MakeVector _returnvalue_2 _returnvalue_2 _returnvalue_2))
      (goto _label Reset))))

(fn ConstructionScript)