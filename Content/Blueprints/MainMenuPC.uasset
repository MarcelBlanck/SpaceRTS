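; MainMenuPC is a player controller, apparently for the main menu of a space RTS.
; On BeginPlay it finds every PlayerPawn actor in the level and possesses each in turn.
; An unconnected Set IPD block would read the interpupillary distance from GameInstanceSpaceRTS and apply it through a stereo console command, but it never runs.
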(event EventBeginPlay
  (Utilities|FlowControl|Sequence
    (:then_1
      ;[1 1 1] Posses Player Pawn
      (bind _outactors (Actor|GetAllActorsOfClass "/Script/SpaceRTS.PlayerPawn"))
      (for _array_element _outactors
        (Pawn|Possess _array_element)))))

(fn ConstructionScript)